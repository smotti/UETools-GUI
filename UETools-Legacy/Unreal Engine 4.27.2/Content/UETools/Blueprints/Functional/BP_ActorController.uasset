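; Free-fly controller that moves and rotates a referenced actor from player input, polling the first player controller, which is re-fetched every second.
; Tick applies mouse and right-stick look with clamped pitch, plus left-stick movement along the actor's axes.
; Movement keys and triggers start and stop fast looping timers that step the location without sweep, with fixed vertical speed.
; The roll-reset key acts on this controller's own rotation, not the referenced actor's.
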(event Custom|Event%20Update%20Running%20PC
  (Variables|Default|SetRunning%20PC (Game|GetPlayerController 0)))

(event Custom|Event%20KeyBack
  (bind _controlled_actor_reference (Variables|Default|GetControlled%20Actor%20Reference))
  (Transformation|SetActorLocation _controlled_actor_reference (+ (Transformation|GetActorLocation _controlled_actor_reference) (* (Math|Vector|GetForwardVector (Transformation|GetActorRotation _controlled_actor_reference)) (* (Variables|Default|GetMovementMultiplier) -1.0))) false false))

(event Custom|Event%20FlyDown
  (bind _controlled_actor_reference (Variables|Default|GetControlled%20Actor%20Reference))
  (Transformation|SetActorLocation _controlled_actor_reference (+ (Transformation|GetActorLocation _controlled_actor_reference) (* (Math|Vector|GetUpVector (Transformation|GetActorRotation _controlled_actor_reference)) -0.4)) false false))

(event Custom|Event%20FlyUp
  (bind _controlled_actor_reference (Variables|Default|GetControlled%20Actor%20Reference))
  (Transformation|SetActorLocation _controlled_actor_reference (+ (Transformation|GetActorLocation _controlled_actor_reference) (* (Math|Vector|GetUpVector (Transformation|GetActorRotation _controlled_actor_reference)) 0.4)) false false))

(event Custom|Event%20KeyForward
  (bind _controlled_actor_reference (Variables|Default|GetControlled%20Actor%20Reference))
  (Transformation|SetActorLocation _controlled_actor_reference (+ (Transformation|GetActorLocation _controlled_actor_reference) (* (Math|Vector|GetForwardVector (Transformation|GetActorRotation _controlled_actor_reference)) (Variables|Default|GetMovementMultiplier))) false false))

(event Custom|Event%20KeyRight
  (bind _controlled_actor_reference (Variables|Default|GetControlled%20Actor%20Reference))
  (Transformation|SetActorLocation _controlled_actor_reference (+ (Transformation|GetActorLocation _controlled_actor_reference) (* (Math|Vector|GetRightVector (Transformation|GetActorRotation _controlled_actor_reference)) (Variables|Default|GetMovementMultiplier))) false false))

(event Custom|Event%20KeyLeft
  (bind _controlled_actor_reference (Variables|Default|GetControlled%20Actor%20Reference))
  (Transformation|SetActorLocation _controlled_actor_reference (+ (Transformation|GetActorLocation _controlled_actor_reference) (* (Math|Vector|GetRightVector (Transformation|GetActorRotation _controlled_actor_reference)) (* (Variables|Default|GetMovementMultiplier) -1.0))) false false))

(event EventTick
  (params (DeltaSeconds :type Float%20%28single-precision%29))
  (bind _self self)
  (bind _key_moveforward (Variables|Default|GetKey_MoveForward))
  (bind _key_moveup (Variables|Default|GetKey_MoveUp))
  (bind _running_pc (Variables|Default|GetRunning%20PC))
  (bind _gamepad_rotation_multiplier (Variables|Default|GetGamepad%20Rotation%20Multiplier))
  (bind _controlled_actor_reference (Variables|Default|GetControlled%20Actor%20Reference))
  (bind _key_movedown (Variables|Default|GetKey_MoveDown))
  (bind _rotationmultiplier (Variables|Default|GetRotationMultiplier))
  (bind _controlled_actor_reference_2 (Variables|Default|GetControlled%20Actor%20Reference))
  (bind _controlled_actor_reference_3 (Variables|Default|GetControlled%20Actor%20Reference))
  (bind _controlled_actor_reference_4 (Variables|Default|GetControlled%20Actor%20Reference))
  (bind _running_pc_2 (Variables|Default|GetRunning%20PC))
  (bind _running_pc_3 (Variables|Default|GetRunning%20PC))
  (bind _running_pc_4 (Variables|Default|GetRunning%20PC))
  (bind _running_pc_5 (Variables|Default|GetRunning%20PC))
  (bind _running_pc_6 (Variables|Default|GetRunning%20PC))
  (bind _key_moveleft (Variables|Default|GetKey_MoveLeft))
  (bind _key_moveright (Variables|Default|GetKey_MoveRight))
  (bind _key_moveback (Variables|Default|GetKey_MoveBack))
  (bind _returnvalue (Transformation|GetActorRotation _controlled_actor_reference_4))
  (bind (_stickx _sticky) (Class|PlayerController|GetInputAnalogStickState _running_pc_3 "CAS_RightStick"))
  (bind _returnvalue_2 (Transformation|GetActorRotation _self))
  (bind _returnvalue_3 (Transformation|GetActorRotation _controlled_actor_reference))
  (bind (_deltax _deltay) (Class|PlayerController|GetInputMouseDelta _running_pc))
  (if (Game|Player|WasInputKeyJustPressed (Variables|Default|GetRunning%20PC) _key_moveforward)
    (bind _returnvalue_4 (Utilities|Time|SetTimerbyEvent (delegate Custom|Event%20KeyForward) 0.001 true)))
  (if (Class|PlayerController|WasInputKeyJustReleased (Variables|Default|GetRunning%20PC) _key_moveforward)
    (Utilities|Time|ClearandInvalidateTimerbyHandle _returnvalue_4))
  (if (Game|Player|WasInputKeyJustPressed (Variables|Default|GetRunning%20PC) _key_moveback)
    (bind _returnvalue_5 (Utilities|Time|SetTimerbyEvent (delegate Custom|Event%20KeyBack) 0.001 true)))
  (if (Class|PlayerController|WasInputKeyJustReleased (Variables|Default|GetRunning%20PC) _key_moveback)
    (Utilities|Time|ClearandInvalidateTimerbyHandle _returnvalue_5))
  (if (Game|Player|WasInputKeyJustPressed (Variables|Default|GetRunning%20PC) _key_moveright)
    (bind _returnvalue_6 (Utilities|Time|SetTimerbyEvent (delegate Custom|Event%20KeyRight) 0.001 true)))
  (if (Class|PlayerController|WasInputKeyJustReleased (Variables|Default|GetRunning%20PC) _key_moveright)
    (Utilities|Time|ClearandInvalidateTimerbyHandle _returnvalue_6))
  (if (Game|Player|WasInputKeyJustPressed (Variables|Default|GetRunning%20PC) _key_moveleft)
    (bind _returnvalue_7 (Utilities|Time|SetTimerbyEvent (delegate Custom|Event%20KeyLeft) 0.001 true)))
  (if (Class|PlayerController|WasInputKeyJustReleased (Variables|Default|GetRunning%20PC) _key_moveleft)
    (Utilities|Time|ClearandInvalidateTimerbyHandle _returnvalue_7))
  (Transformation|SetActorRotation _controlled_actor_reference (Math|Rotator|MakeRotator (.roll _returnvalue_3) (Math|Float|Clamp(Float) (+ (.pitch _returnvalue_3) (* _deltay _rotationmultiplier)) -89.0 89.0) (+ (.yaw _returnvalue_3) (* _deltax _rotationmultiplier))))
  (Transformation|SetActorLocation _controlled_actor_reference_3 (+ (Transformation|GetActorLocation _controlled_actor_reference_3) (* (Math|Vector|GetRightVector (Transformation|GetActorRotation _controlled_actor_reference_3)) (* (Variables|Default|GetGamepad%20Movement%20Multiplier) (.StickX (Class|PlayerController|GetInputAnalogStickState (Variables|Default|GetRunning%20PC) "CAS_LeftStick"))))) false false)
  (Transformation|SetActorLocation _controlled_actor_reference_2 (+ (Transformation|GetActorLocation _controlled_actor_reference_2) (* (Math|Vector|GetForwardVector (Transformation|GetActorRotation _controlled_actor_reference_2)) (* (Variables|Default|GetGamepad%20Movement%20Multiplier) (.StickY (Class|PlayerController|GetInputAnalogStickState (Variables|Default|GetRunning%20PC) "CAS_LeftStick"))))) false false)
  (Transformation|SetActorRotation _controlled_actor_reference_4 (Math|Rotator|MakeRotator (.roll _returnvalue) (Math|Float|Clamp(Float) (+ (.pitch _returnvalue) (* (* _sticky _gamepad_rotation_multiplier) -1.0)) -89.0 89.0) (+ (.yaw _returnvalue) (* _stickx _gamepad_rotation_multiplier))))
  (if (or (Game|Player|WasInputKeyJustPressed _running_pc_2 "Gamepad_LeftTriggerAxis") (Game|Player|WasInputKeyJustPressed _running_pc_2 _key_movedown))
    (bind _returnvalue_8 (Utilities|Time|SetTimerbyEvent (delegate Custom|Event%20FlyDown) 0.001 true)))
  (if (or (Class|PlayerController|WasInputKeyJustReleased _running_pc_4 "Gamepad_LeftTriggerAxis") (Class|PlayerController|WasInputKeyJustReleased _running_pc_4 _key_movedown))
    (Utilities|Time|ClearandInvalidateTimerbyHandle _returnvalue_8))
  (if (or (Game|Player|WasInputKeyJustPressed _running_pc_5 "Gamepad_RightTriggerAxis") (Game|Player|WasInputKeyJustPressed _running_pc_5 _key_moveup))
    (bind _returnvalue_9 (Utilities|Time|SetTimerbyEvent (delegate Custom|Event%20FlyUp) 0.001 true)))
  (if (or (Class|PlayerController|WasInputKeyJustReleased _running_pc_6 "Gamepad_RightTriggerAxis") (Class|PlayerController|WasInputKeyJustReleased _running_pc_6 _key_moveup))
    (Utilities|Time|ClearandInvalidateTimerbyHandle _returnvalue_9))
  (if (Game|Player|WasInputKeyJustPressed (Variables|Default|GetRunning%20PC) (Variables|Default|GetKey_ResetRoll))
    (Transformation|SetActorRotation _self (Math|Rotator|MakeRotator 0.0 (.pitch _returnvalue_2) (.yaw _returnvalue_2)))))

(event EventBeginPlay
  (Utilities|Time|SetTimerbyEvent (delegate Custom|Event%20Update%20Running%20PC) 1.0 true))

(fn ConstructionScript)