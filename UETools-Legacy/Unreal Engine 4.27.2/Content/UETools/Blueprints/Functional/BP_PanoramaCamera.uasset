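; BP_PanoramaCamera is a UETools camera actor that captures a 360-degree panorama as a series of promo screenshots.
; CreatePanoramaShot takes a first screenshot through the cheat manager, then a delayed loop steps the actor's yaw by RotationStep and shoots again, pausing between shots to cover the full circle.
; When the loop completes, it notifies the cheat manager that the panorama has been created.
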(event Custom|Event%20Create%20Panorama%20Shot
  (params (Quality%20Level :type Integer) (Rotation%20Step :type Float%20%28single-precision%29))
  (bind _self self)
  (Utilities|FlowControl|Sequence
    (:then_0
      (Default|UEToolsPromoScreenshot (Variables|Default|GetCheat%20Manager%20Reference) Quality%20Level :!label _label))
    (:then_1
      (Utilities|ForLoopwithDelay 0 (- (Math|Float|Round (/ 3.6e+02 Rotation%20Step)) 2) 2.0
        (:Loop%20Body
          (Transformation|SetActorRotation _self (Math|Rotator|MakeRotator 0.0 0.0 (+ (.yaw (Transformation|GetActorRotation _self)) Rotation%20Step)))
          (goto _label))
        (:Completed
          (Default|EventF::PanoramaScreenShotCreated (Variables|Default|GetCheat%20Manager%20Reference)))))))

(fn ConstructionScript)