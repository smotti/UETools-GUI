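; BPC_Outline is a component that swaps the material on its owner's static meshes through Enable and Disable events, apparently as an outline toggle.
; Enable caches materials in a map keyed by mesh component, keeping one per mesh, and creates a dynamic TextureBasedMorphDemo instance on slot 0.
; Disable looks up each mesh's cached material and sets it back on slot 0 only.
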(event Custom|Event%20Disable
  (for _array_element (Actor|GetComponentsByClass (Components|GetOwner self) "/Script/Engine.StaticMeshComponent")
    (Rendering|Material|SetMaterial _array_element 0 (.Value (Utilities|Map|Find (Variables|Default|GetStatic%20Meshes) _array_element)))))

(event Custom|Event%20Enable
  (for _array_element (Actor|GetComponentsByClass (Components|GetOwner self) "/Script/Engine.StaticMeshComponent")
    (for _array_element_2 (Rendering|Material|GetMaterials _array_element)
      (Utilities|Map|Add (Variables|Default|GetStatic%20Meshes) _array_element _array_element_2)
      (Rendering|Material|CreateDynamicMaterialInstance _array_element 0 "/Engine/Functions/Engine_MaterialFunctions02/ExampleContent/TextureBasedWPO/TextureBasedMorphDemo.TextureBasedMorphDemo" "None" :!class /Script/Engine.PrimitiveComponent))))