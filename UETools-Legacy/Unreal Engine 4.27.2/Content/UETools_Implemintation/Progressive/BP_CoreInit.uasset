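; BP_CoreInit bootstraps UETools in a running game from a Settings object it spawns on first Tick.
; It reuses an existing WBP_UEToolsCore widget or creates one with those settings.
; A looping timer waits for the cheat manager unless the core already existed.
; It then spawns modding actors from class paths, runs auto-exec console commands, and optionally sets GameDefaultMap and auto-travels to the configured level.
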(event Custom|Event%20OnCheatManagerCreated
  (bind _settingsobjectreference (Variables|Default|GetSettingsObjectReference))
  (if (or (Variables|/Game/UETools_Implemintation/WBP_UEToolsCore.WBP_UEToolsCore_C|GetbWasCheatManagerConstructed (Variables|Default|GetCoreReference)) (Variables|Default|GetCoreWasAlreadyConstructed))
    (CallFunction|ProcessModding)
    (CallFunction|ProcessAutoExecCommands)
    (Utilities|Time|ClearandInvalidateTimerbyHandle (stale EventTick _returnvalue_3))
    (Utilities|FlowControl|Sequence
      (:then_0
        (if (Variables|/Game/UETools_Implemintation/Progressive/Settings.Settings_C|GetbAutoTravelRestoreGameDefaultMap (Variables|Default|GetSettingsObjectReference))
          (Variables|/Script/EngineSettings.GameMapsSettings|SetGameDefaultMap (Class|GameMapsSettings|GetGameMapsSettings) (Utilities|MakeSoftObjectPath (CallFunction|GetGameDefaultMap)))))
      (:then_1
        (if (Variables|/Game/UETools_Implemintation/Progressive/Settings.Settings_C|GetbEnableAutoTravel _settingsobjectreference)
          (Utilities|FlowControl|Delay (Variables|/Game/UETools_Implemintation/Progressive/Settings.Settings_C|GetAutoTravelDelay _settingsobjectreference))
          (Game|OpenLevel(byName) (Variables|/Game/UETools_Implemintation/Progressive/Settings.Settings_C|GetAutoTravelLevelName _settingsobjectreference) (Variables|/Game/UETools_Implemintation/Progressive/Settings.Settings_C|GetbAutoTravelAbsolute _settingsobjectreference) (Variables|/Game/UETools_Implemintation/Progressive/Settings.Settings_C|GetAutoTravelOptions _settingsobjectreference)))))))

(event EventTick
  (params (DeltaSeconds :type Float%20%28single-precision%29))
  (Utilities|FlowControl|DoOnce false
    (:Completed
      (Utilities|FlowControl|Sequence
        (:then_0
          (bind _returnvalue (CallFunction|SpawnObject "/Game/UETools_Implemintation/Progressive/Settings.Settings_C" self))
          (bind _assettings (Utilities|Casting|CastToSettings _returnvalue))
          (Variables|Default|SetSettingsObjectReference _assettings))
        (:then_1
          (bind _foundwidgets (Widget|GetAllWidgetsOfClass "/Game/UETools_Implemintation/WBP_UEToolsCore.WBP_UEToolsCore_C" true))
          (Utilities|IsValid (Utilities|Array|Get(acopy) _foundwidgets)
            (:Is%20Valid
              (Variables|Default|SetCoreReference (Utilities|Array|Get(acopy) _foundwidgets))
              (Variables|Default|SetCoreWasAlreadyConstructed true))
            (:Is%20Not%20Valid
              (bind _returnvalue_2 (UserInterface|CreateWidget "/Game/UETools_Implemintation/WBP_UEToolsCore.WBP_UEToolsCore_C" 0 (Variables|/Game/UETools_Implemintation/Progressive/Settings.Settings_C|GetCoreValidationDelay (Variables|Default|GetSettingsObjectReference)) (Variables|/Game/UETools_Implemintation/Progressive/Settings.Settings_C|GetbCreateDebugMappings (Variables|Default|GetSettingsObjectReference)) (CallFunction|GetDebugMappingsMap) (Variables|/Game/UETools_Implemintation/Progressive/Settings.Settings_C|GetHighResScreenshotResolution (Variables|Default|GetSettingsObjectReference)) (Variables|/Game/UETools_Implemintation/Progressive/Settings.Settings_C|GetbConstructConsole (Variables|Default|GetSettingsObjectReference)) (Variables|/Game/UETools_Implemintation/Progressive/Settings.Settings_C|GetbForceDefaultConsoleClass (Variables|Default|GetSettingsObjectReference)) (Variables|/Game/UETools_Implemintation/Progressive/Settings.Settings_C|GetbCreateConsoleMappings (Variables|Default|GetSettingsObjectReference)) (Variables|/Game/UETools_Implemintation/Progressive/Settings.Settings_C|GetbConstructCheatManager (Variables|Default|GetSettingsObjectReference)) (Variables|/Game/UETools_Implemintation/Progressive/Settings.Settings_C|GetbForceDefaultCheatManagerClass (Variables|Default|GetSettingsObjectReference)) (Variables|/Game/UETools_Implemintation/Progressive/Settings.Settings_C|GetbManualConstructCheatManager (Variables|Default|GetSettingsObjectReference))))
              (UserInterface|Viewport|AddtoViewport _returnvalue_2 0)
              (Variables|Default|SetCoreReference _returnvalue_2))))
        (:then_2
          (bind _returnvalue_3 (Utilities|Time|SetTimerbyEvent (delegate Custom|Event%20OnCheatManagerCreated) 0.1 true)))))))

(fn ConstructionScript)

(fn ProcessModding
  (bind _settingsobjectreference (Variables|Default|GetSettingsObjectReference))
  (if (Variables|/Game/UETools_Implemintation/Progressive/Settings.Settings_C|GetbModdingSupportEnabled _settingsobjectreference)
    (for _array_element (Utilities|Array|MakeArray (Variables|/Game/UETools_Implemintation/Progressive/Settings.Settings_C|GetModdingActorPath_01 _settingsobjectreference) (Variables|/Game/UETools_Implemintation/Progressive/Settings.Settings_C|GetModdingActorPath_02 _settingsobjectreference) (Variables|/Game/UETools_Implemintation/Progressive/Settings.Settings_C|GetModdingActorPath_03 _settingsobjectreference) (Variables|/Game/UETools_Implemintation/Progressive/Settings.Settings_C|GetModdingActorPath_04 _settingsobjectreference) (Variables|/Game/UETools_Implemintation/Progressive/Settings.Settings_C|GetModdingActorPath_05 _settingsobjectreference) (Variables|/Game/UETools_Implemintation/Progressive/Settings.Settings_C|GetModdingActorPath_06 _settingsobjectreference) (Variables|/Game/UETools_Implemintation/Progressive/Settings.Settings_C|GetModdingActorPath_07 _settingsobjectreference) (Variables|/Game/UETools_Implemintation/Progressive/Settings.Settings_C|GetModdingActorPath_08 _settingsobjectreference) (Variables|/Game/UETools_Implemintation/Progressive/Settings.Settings_C|GetModdingActorPath_09 _settingsobjectreference) (Variables|/Game/UETools_Implemintation/Progressive/Settings.Settings_C|GetModdingActorPath_10 _settingsobjectreference) (Variables|/Game/UETools_Implemintation/Progressive/Settings.Settings_C|GetModdingActorPath_11 _settingsobjectreference) (Variables|/Game/UETools_Implemintation/Progressive/Settings.Settings_C|GetModdingActorPath_12 _settingsobjectreference) (Variables|/Game/UETools_Implemintation/Progressive/Settings.Settings_C|GetModdingActorPath_13 _settingsobjectreference) (Variables|/Game/UETools_Implemintation/Progressive/Settings.Settings_C|GetModdingActorPath_14 _settingsobjectreference) (Variables|/Game/UETools_Implemintation/Progressive/Settings.Settings_C|GetModdingActorPath_15 _settingsobjectreference) (Variables|/Game/UETools_Implemintation/Progressive/Settings.Settings_C|GetModdingActorPath_16 _settingsobjectreference) (Variables|/Game/UETools_Implemintation/Progressive/Settings.Settings_C|GetModdingActorPath_17 _settingsobjectreference) (Variables|/Game/UETools_Implemintation/Progressive/Settings.Settings_C|GetModdingActorPath_18 _settingsobjectreference) (Variables|/Game/UETools_Implemintation/Progressive/Settings.Settings_C|GetModdingActorPath_19 _settingsobjectreference) (Variables|/Game/UETools_Implemintation/Progressive/Settings.Settings_C|GetModdingActorPath_20 _settingsobjectreference) (Variables|/Game/UETools_Implemintation/Progressive/Settings.Settings_C|GetModdingActorPath_21 _settingsobjectreference) (Variables|/Game/UETools_Implemintation/Progressive/Settings.Settings_C|GetModdingActorPath_22 _settingsobjectreference) (Variables|/Game/UETools_Implemintation/Progressive/Settings.Settings_C|GetModdingActorPath_23 _settingsobjectreference) (Variables|/Game/UETools_Implemintation/Progressive/Settings.Settings_C|GetModdingActorPath_24 _settingsobjectreference))
      (bind _returnvalue (Utilities|LoadClassAssetBlocking (Class|KismetSystemLibrary|ToSoftClassRef(SoftClassPath) (Class|KismetSystemLibrary|MakeSoftClassPath _array_element))))
      (if (Utilities|IsValidClass _returnvalue)
        (bind _asactor (Utilities|Casting|CastToActorClass _returnvalue))
        (Game|SpawnActorfromClass _asactor (Math|Transform|MakeTransform "0, 0, 0" "0, 0, 0" "1,1,1") "Undefined" 0 0)))))

(fn GetDebugMappingsMap
  (bind _settingsobjectreference (Variables|Default|GetSettingsObjectReference))
  (return (Utilities|Map|MakeMap "NewEnumerator0" (Variables|/Game/UETools_Implemintation/Progressive/Settings.Settings_C|GetDebugMapping_ToggleFullScreen _settingsobjectreference) "NewEnumerator1" (Variables|/Game/UETools_Implemintation/Progressive/Settings.Settings_C|GetDebugMapping_Screenshot _settingsobjectreference) "NewEnumerator2" (Variables|/Game/UETools_Implemintation/Progressive/Settings.Settings_C|GetDebugMapping_ScreenshotUI _settingsobjectreference) "NewEnumerator3" (Variables|/Game/UETools_Implemintation/Progressive/Settings.Settings_C|GetDebugMapping_HighResScreenshot _settingsobjectreference) "NewEnumerator4" (Variables|/Game/UETools_Implemintation/Progressive/Settings.Settings_C|GetDebugMapping_PreviousDebugTarget _settingsobjectreference) "NewEnumerator5" (Variables|/Game/UETools_Implemintation/Progressive/Settings.Settings_C|GetDebugMapping_NextDebugTarget _settingsobjectreference) "NewEnumerator6" (Variables|/Game/UETools_Implemintation/Progressive/Settings.Settings_C|GetDebugMapping_ToggleDebugStats _settingsobjectreference) "NewEnumerator9" (Variables|/Game/UETools_Implemintation/Progressive/Settings.Settings_C|GetDebugMapping_PreviousViewMode _settingsobjectreference) "NewEnumerator7" (Variables|/Game/UETools_Implemintation/Progressive/Settings.Settings_C|GetDebugMapping_NextViewMode _settingsobjectreference))))

(fn ProcessAutoExecCommands
  (bind _settingsobjectreference (Variables|Default|GetSettingsObjectReference))
  (for _array_element (Utilities|Array|MakeArray (Variables|/Game/UETools_Implemintation/Progressive/Settings.Settings_C|GetAutoExecCommand_01 _settingsobjectreference) (Variables|/Game/UETools_Implemintation/Progressive/Settings.Settings_C|GetAutoExecCommand_02 _settingsobjectreference) (Variables|/Game/UETools_Implemintation/Progressive/Settings.Settings_C|GetAutoExecCommand_03 _settingsobjectreference) (Variables|/Game/UETools_Implemintation/Progressive/Settings.Settings_C|GetAutoExecCommand_04 _settingsobjectreference) (Variables|/Game/UETools_Implemintation/Progressive/Settings.Settings_C|GetAutoExecCommand_05 _settingsobjectreference) (Variables|/Game/UETools_Implemintation/Progressive/Settings.Settings_C|GetAutoExecCommand_06 _settingsobjectreference) (Variables|/Game/UETools_Implemintation/Progressive/Settings.Settings_C|GetAutoExecCommand_07 _settingsobjectreference) (Variables|/Game/UETools_Implemintation/Progressive/Settings.Settings_C|GetAutoExecCommand_08 _settingsobjectreference) (Variables|/Game/UETools_Implemintation/Progressive/Settings.Settings_C|GetAutoExecCommand_09 _settingsobjectreference) (Variables|/Game/UETools_Implemintation/Progressive/Settings.Settings_C|GetAutoExecCommand_10 _settingsobjectreference) (Variables|/Game/UETools_Implemintation/Progressive/Settings.Settings_C|GetAutoExecCommand_11 _settingsobjectreference) (Variables|/Game/UETools_Implemintation/Progressive/Settings.Settings_C|GetAutoExecCommand_12 _settingsobjectreference))
    (if (not (Utilities|Array|IsEmpty _array_element))
      (Development|ExecuteConsoleCommand _array_element 0))))

(fn GetGameDefaultMap
  (bind _settingsobjectreference (Variables|Default|GetSettingsObjectReference))
  (bind _autotravellevelname (Variables|/Game/UETools_Implemintation/Progressive/Settings.Settings_C|GetAutoTravelLevelName _settingsobjectreference))
  (bind _returnvalue (Utilities|String|ToString(Name) _autotravellevelname))
  (return (Utilities|String|ToString(Text) (Utilities|Text|FormatText "{FullPathIncomplete}.{FullPathSecond}" _returnvalue (.RightS (Utilities|String|Split _returnvalue "/" "IgnoreCase" "FromEnd"))))))