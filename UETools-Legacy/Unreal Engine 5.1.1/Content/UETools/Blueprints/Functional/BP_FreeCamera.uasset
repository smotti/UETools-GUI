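; Free-fly camera actor that accepts keyboard, mouse and gamepad control only while it is the view target.
; Tick polls a player controller reference, refreshed every second, for stick movement, mouse or stick rotation with clamped pitch, and roll reset.
; Movement keys and triggers start fast looping timers that offset the actor along its local axes without sweeping.
; Releasing an input clears its timer, and losing view target clears them all.
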(event Custom|Event%20Update%20Running%20PC
  (Variables|Default|SetRunningPC (Game|GetPlayerController 0)))

(event Custom|Event%20KeyBack
  (bind _self self)
  (Transformation|SetActorLocation _self (+ (Transformation|GetActorLocation _self) (* (Math|Vector|GetForwardVector (Transformation|GetActorRotation _self)) (* (Variables|Default|GetMovement%20Multiplier) -1.0))) false false))

(event Custom|Event%20FlyDown
  (bind _self self)
  (Transformation|SetActorLocation _self (+ (Transformation|GetActorLocation _self) (* (Math|Vector|GetUpVector (Transformation|GetActorRotation _self)) (Variables|Default|GetDown%20Multiplier))) false false))

(event Custom|Event%20ForceStop_KeyLeft
  (bind _self self)
  (bind _self_2 self)
  (bind _self_3 self)
  (bind _self_4 self)
  (bind _self_5 self)
  (bind _runningpc (Variables|Default|GetRunningPC))
  (bind _key_moveup (Variables|Default|GetKey_MoveUp))
  (bind _key_movedown (Variables|Default|GetKey_MoveDown))
  (bind _runningpc_2 (Variables|Default|GetRunningPC))
  (bind _rotation_multiplier (Variables|Default|GetRotation%20Multiplier))
  (bind _runningpc_3 (Variables|Default|GetRunningPC))
  (bind _gamepad_rotation_multiplier (Variables|Default|GetGamepad%20Rotation%20Multiplier))
  (bind _runningpc_4 (Variables|Default|GetRunningPC))
  (bind _runningpc_5 (Variables|Default|GetRunningPC))
  (bind _runningpc_6 (Variables|Default|GetRunningPC))
  (bind _returnvalue (Transformation|GetActorRotation _self_2))
  (bind (_stickx _sticky) (Class|PlayerController|GetInputAnalogStickState _runningpc "CAS_RightStick"))
  (bind _returnvalue_2 (Transformation|GetActorRotation _self_3))
  (bind _returnvalue_3 (Transformation|GetActorRotation _self_4))
  (bind (_deltax _deltay) (Class|PlayerController|GetInputMouseDelta _runningpc_2))
  (Utilities|Time|ClearandInvalidateTimerbyHandle (stale Custom|Event%20ForceStop_KeyBack _returnvalue_5))
  (Transformation|SetActorRotation _self_4 (Math|Rotator|MakeRotator (.roll _returnvalue_3) (Math|Float|Clamp(Float) (+ (.pitch _returnvalue_3) (* _deltay _rotation_multiplier)) -89.0 89.0) (+ (.yaw _returnvalue_3) (* _deltax _rotation_multiplier))))
  (Transformation|SetActorLocation _self_5 (+ (Transformation|GetActorLocation _self_5) (* (Math|Vector|GetRightVector (Transformation|GetActorRotation _self_5)) (* (Variables|Default|GetGamepad%20Movement%20Multiplier) (.StickX (Class|PlayerController|GetInputAnalogStickState (Variables|Default|GetRunningPC) "CAS_LeftStick"))))) false false)
  (Transformation|SetActorLocation _self (+ (Transformation|GetActorLocation _self) (* (Math|Vector|GetForwardVector (Transformation|GetActorRotation _self)) (* (Variables|Default|GetGamepad%20Movement%20Multiplier) (.StickY (Class|PlayerController|GetInputAnalogStickState (Variables|Default|GetRunningPC) "CAS_LeftStick"))))) false false)
  (Transformation|SetActorRotation _self_2 (Math|Rotator|MakeRotator (.roll _returnvalue) (Math|Float|Clamp(Float) (+ (.pitch _returnvalue) (* (* _sticky _gamepad_rotation_multiplier) -1.0)) -89.0 89.0) (+ (.yaw _returnvalue) (* _stickx _gamepad_rotation_multiplier))))
  (if (or (Game|Player|WasInputKeyJustPressed _runningpc_4 "Gamepad_LeftTriggerAxis") (Game|Player|WasInputKeyJustPressed _runningpc_4 _key_movedown))
    (bind _returnvalue_4 (Utilities|Time|SetTimerbyEvent (delegate Custom|Event%20FlyDown) 0.001 true)))
  (if (or (Class|PlayerController|WasInputKeyJustReleased _runningpc_6 "Gamepad_LeftTriggerAxis") (Class|PlayerController|WasInputKeyJustReleased _runningpc_6 _key_movedown))
    (Utilities|Time|ClearandInvalidateTimerbyHandle _returnvalue_4))
  (if (or (Game|Player|WasInputKeyJustPressed _runningpc_5 "Gamepad_RightTriggerAxis") (Game|Player|WasInputKeyJustPressed _runningpc_5 _key_moveup))
    (bind _returnvalue_5 (Utilities|Time|SetTimerbyEvent (delegate Custom|Event%20FlyUp) 0.001 true)))
  (if (or (Class|PlayerController|WasInputKeyJustReleased _runningpc_3 "Gamepad_RightTriggerAxis") (Class|PlayerController|WasInputKeyJustReleased _runningpc_3 _key_moveup))
    (Utilities|Time|ClearandInvalidateTimerbyHandle _returnvalue_5))
  (if (Game|Player|WasInputKeyJustPressed (Variables|Default|GetRunningPC) (Variables|Default|GetKey_ResetRoll))
    (Transformation|SetActorRotation _self_3 (Math|Rotator|MakeRotator 0.0 (.pitch _returnvalue_2) (.yaw _returnvalue_2)))))

(event Custom|Event%20ForceStop_FlyDown
  (bind _self self)
  (bind _key_moveup (Variables|Default|GetKey_MoveUp))
  (bind _runningpc (Variables|Default|GetRunningPC))
  (bind _runningpc_2 (Variables|Default|GetRunningPC))
  (bind _returnvalue (Transformation|GetActorRotation _self))
  (Utilities|Time|ClearandInvalidateTimerbyHandle (stale Custom|Event%20ForceStop_KeyLeft _returnvalue_4))
  (if (or (Game|Player|WasInputKeyJustPressed _runningpc_2 "Gamepad_RightTriggerAxis") (Game|Player|WasInputKeyJustPressed _runningpc_2 _key_moveup))
    (bind _returnvalue_2 (Utilities|Time|SetTimerbyEvent (delegate Custom|Event%20FlyUp) 0.001 true)))
  (if (or (Class|PlayerController|WasInputKeyJustReleased _runningpc "Gamepad_RightTriggerAxis") (Class|PlayerController|WasInputKeyJustReleased _runningpc _key_moveup))
    (Utilities|Time|ClearandInvalidateTimerbyHandle _returnvalue_2))
  (if (Game|Player|WasInputKeyJustPressed (Variables|Default|GetRunningPC) (Variables|Default|GetKey_ResetRoll))
    (Transformation|SetActorRotation _self (Math|Rotator|MakeRotator 0.0 (.pitch _returnvalue) (.yaw _returnvalue)))))

(event Custom|Event%20ForceStop_FlyUp
  (bind _self self)
  (bind _returnvalue (Transformation|GetActorRotation _self))
  (Utilities|Time|ClearandInvalidateTimerbyHandle (stale Custom|Event%20ForceStop_KeyLeft _returnvalue_5))
  (if (Game|Player|WasInputKeyJustPressed (Variables|Default|GetRunningPC) (Variables|Default|GetKey_ResetRoll))
    (Transformation|SetActorRotation _self (Math|Rotator|MakeRotator 0.0 (.pitch _returnvalue) (.yaw _returnvalue)))))

(event Custom|Event%20FlyUp
  (bind _self self)
  (Transformation|SetActorLocation _self (+ (Transformation|GetActorLocation _self) (* (Math|Vector|GetUpVector (Transformation|GetActorRotation _self)) (Variables|Default|GetUp%20Multiplier))) false false))

(event Custom|Event%20ForceStop_KeyBack
  (bind _self self)
  (bind _self_2 self)
  (bind _self_3 self)
  (bind _self_4 self)
  (bind _self_5 self)
  (bind _key_moveright (Variables|Default|GetKey_MoveRight))
  (bind _key_moveleft (Variables|Default|GetKey_MoveLeft))
  (bind _runningpc (Variables|Default|GetRunningPC))
  (bind _key_moveup (Variables|Default|GetKey_MoveUp))
  (bind _key_movedown (Variables|Default|GetKey_MoveDown))
  (bind _runningpc_2 (Variables|Default|GetRunningPC))
  (bind _rotation_multiplier (Variables|Default|GetRotation%20Multiplier))
  (bind _runningpc_3 (Variables|Default|GetRunningPC))
  (bind _gamepad_rotation_multiplier (Variables|Default|GetGamepad%20Rotation%20Multiplier))
  (bind _runningpc_4 (Variables|Default|GetRunningPC))
  (bind _runningpc_5 (Variables|Default|GetRunningPC))
  (bind _runningpc_6 (Variables|Default|GetRunningPC))
  (bind _returnvalue (Transformation|GetActorRotation _self_2))
  (bind (_stickx _sticky) (Class|PlayerController|GetInputAnalogStickState _runningpc "CAS_RightStick"))
  (bind _returnvalue_2 (Transformation|GetActorRotation _self_3))
  (bind _returnvalue_3 (Transformation|GetActorRotation _self_4))
  (bind (_deltax _deltay) (Class|PlayerController|GetInputMouseDelta _runningpc_2))
  (Utilities|Time|ClearandInvalidateTimerbyHandle (stale Custom|Event%20ForceStop_KeyForward _returnvalue_4))
  (if (Game|Player|WasInputKeyJustPressed (Variables|Default|GetRunningPC) _key_moveright)
    (bind _returnvalue_4 (Utilities|Time|SetTimerbyEvent (delegate Custom|Event%20KeyRight) 0.001 true)))
  (if (Class|PlayerController|WasInputKeyJustReleased (Variables|Default|GetRunningPC) _key_moveright)
    (Utilities|Time|ClearandInvalidateTimerbyHandle _returnvalue_4))
  (if (Game|Player|WasInputKeyJustPressed (Variables|Default|GetRunningPC) _key_moveleft)
    (bind _returnvalue_5 (Utilities|Time|SetTimerbyEvent (delegate Custom|Event%20KeyLeft) 0.001 true)))
  (if (Class|PlayerController|WasInputKeyJustReleased (Variables|Default|GetRunningPC) _key_moveleft)
    (Utilities|Time|ClearandInvalidateTimerbyHandle _returnvalue_5))
  (Transformation|SetActorRotation _self_4 (Math|Rotator|MakeRotator (.roll _returnvalue_3) (Math|Float|Clamp(Float) (+ (.pitch _returnvalue_3) (* _deltay _rotation_multiplier)) -89.0 89.0) (+ (.yaw _returnvalue_3) (* _deltax _rotation_multiplier))))
  (Transformation|SetActorLocation _self_5 (+ (Transformation|GetActorLocation _self_5) (* (Math|Vector|GetRightVector (Transformation|GetActorRotation _self_5)) (* (Variables|Default|GetGamepad%20Movement%20Multiplier) (.StickX (Class|PlayerController|GetInputAnalogStickState (Variables|Default|GetRunningPC) "CAS_LeftStick"))))) false false)
  (Transformation|SetActorLocation _self (+ (Transformation|GetActorLocation _self) (* (Math|Vector|GetForwardVector (Transformation|GetActorRotation _self)) (* (Variables|Default|GetGamepad%20Movement%20Multiplier) (.StickY (Class|PlayerController|GetInputAnalogStickState (Variables|Default|GetRunningPC) "CAS_LeftStick"))))) false false)
  (Transformation|SetActorRotation _self_2 (Math|Rotator|MakeRotator (.roll _returnvalue) (Math|Float|Clamp(Float) (+ (.pitch _returnvalue) (* (* _sticky _gamepad_rotation_multiplier) -1.0)) -89.0 89.0) (+ (.yaw _returnvalue) (* _stickx _gamepad_rotation_multiplier))))
  (if (or (Game|Player|WasInputKeyJustPressed _runningpc_4 "Gamepad_LeftTriggerAxis") (Game|Player|WasInputKeyJustPressed _runningpc_4 _key_movedown))
    (bind _returnvalue_6 (Utilities|Time|SetTimerbyEvent (delegate Custom|Event%20FlyDown) 0.001 true)))
  (if (or (Class|PlayerController|WasInputKeyJustReleased _runningpc_6 "Gamepad_LeftTriggerAxis") (Class|PlayerController|WasInputKeyJustReleased _runningpc_6 _key_movedown))
    (Utilities|Time|ClearandInvalidateTimerbyHandle _returnvalue_6))
  (if (or (Game|Player|WasInputKeyJustPressed _runningpc_5 "Gamepad_RightTriggerAxis") (Game|Player|WasInputKeyJustPressed _runningpc_5 _key_moveup))
    (bind _returnvalue_7 (Utilities|Time|SetTimerbyEvent (delegate Custom|Event%20FlyUp) 0.001 true)))
  (if (or (Class|PlayerController|WasInputKeyJustReleased _runningpc_3 "Gamepad_RightTriggerAxis") (Class|PlayerController|WasInputKeyJustReleased _runningpc_3 _key_moveup))
    (Utilities|Time|ClearandInvalidateTimerbyHandle _returnvalue_7))
  (if (Game|Player|WasInputKeyJustPressed (Variables|Default|GetRunningPC) (Variables|Default|GetKey_ResetRoll))
    (Transformation|SetActorRotation _self_3 (Math|Rotator|MakeRotator 0.0 (.pitch _returnvalue_2) (.yaw _returnvalue_2)))))

(event Custom|Event%20KeyForward
  (bind _self self)
  (Transformation|SetActorLocation _self (+ (Transformation|GetActorLocation _self) (* (Math|Vector|GetForwardVector (Transformation|GetActorRotation _self)) (Variables|Default|GetMovement%20Multiplier))) false false))

(event Custom|Event%20ForceStop_KeyForward
  (bind _self self)
  (bind _self_2 self)
  (bind _self_3 self)
  (bind _self_4 self)
  (bind _self_5 self)
  (bind _key_moveback (Variables|Default|GetKey_MoveBack))
  (bind _key_moveright (Variables|Default|GetKey_MoveRight))
  (bind _key_moveleft (Variables|Default|GetKey_MoveLeft))
  (bind _runningpc (Variables|Default|GetRunningPC))
  (bind _key_moveup (Variables|Default|GetKey_MoveUp))
  (bind _key_movedown (Variables|Default|GetKey_MoveDown))
  (bind _runningpc_2 (Variables|Default|GetRunningPC))
  (bind _rotation_multiplier (Variables|Default|GetRotation%20Multiplier))
  (bind _runningpc_3 (Variables|Default|GetRunningPC))
  (bind _gamepad_rotation_multiplier (Variables|Default|GetGamepad%20Rotation%20Multiplier))
  (bind _runningpc_4 (Variables|Default|GetRunningPC))
  (bind _runningpc_5 (Variables|Default|GetRunningPC))
  (bind _runningpc_6 (Variables|Default|GetRunningPC))
  (bind _returnvalue (Transformation|GetActorRotation _self_2))
  (bind (_stickx _sticky) (Class|PlayerController|GetInputAnalogStickState _runningpc "CAS_RightStick"))
  (bind _returnvalue_2 (Transformation|GetActorRotation _self_3))
  (bind _returnvalue_3 (Transformation|GetActorRotation _self_4))
  (bind (_deltax _deltay) (Class|PlayerController|GetInputMouseDelta _runningpc_2))
  (Utilities|Time|ClearandInvalidateTimerbyHandle (stale EventTick _returnvalue_4))
  (if (Game|Player|WasInputKeyJustPressed (Variables|Default|GetRunningPC) _key_moveback)
    (bind _returnvalue_4 (Utilities|Time|SetTimerbyEvent (delegate Custom|Event%20KeyBack) 0.001 true)))
  (if (Class|PlayerController|WasInputKeyJustReleased (Variables|Default|GetRunningPC) _key_moveback)
    (Utilities|Time|ClearandInvalidateTimerbyHandle _returnvalue_4))
  (if (Game|Player|WasInputKeyJustPressed (Variables|Default|GetRunningPC) _key_moveright)
    (bind _returnvalue_5 (Utilities|Time|SetTimerbyEvent (delegate Custom|Event%20KeyRight) 0.001 true)))
  (if (Class|PlayerController|WasInputKeyJustReleased (Variables|Default|GetRunningPC) _key_moveright)
    (Utilities|Time|ClearandInvalidateTimerbyHandle _returnvalue_5))
  (if (Game|Player|WasInputKeyJustPressed (Variables|Default|GetRunningPC) _key_moveleft)
    (bind _returnvalue_6 (Utilities|Time|SetTimerbyEvent (delegate Custom|Event%20KeyLeft) 0.001 true)))
  (if (Class|PlayerController|WasInputKeyJustReleased (Variables|Default|GetRunningPC) _key_moveleft)
    (Utilities|Time|ClearandInvalidateTimerbyHandle _returnvalue_6))
  (Transformation|SetActorRotation _self_4 (Math|Rotator|MakeRotator (.roll _returnvalue_3) (Math|Float|Clamp(Float) (+ (.pitch _returnvalue_3) (* _deltay _rotation_multiplier)) -89.0 89.0) (+ (.yaw _returnvalue_3) (* _deltax _rotation_multiplier))))
  (Transformation|SetActorLocation _self_5 (+ (Transformation|GetActorLocation _self_5) (* (Math|Vector|GetRightVector (Transformation|GetActorRotation _self_5)) (* (Variables|Default|GetGamepad%20Movement%20Multiplier) (.StickX (Class|PlayerController|GetInputAnalogStickState (Variables|Default|GetRunningPC) "CAS_LeftStick"))))) false false)
  (Transformation|SetActorLocation _self (+ (Transformation|GetActorLocation _self) (* (Math|Vector|GetForwardVector (Transformation|GetActorRotation _self)) (* (Variables|Default|GetGamepad%20Movement%20Multiplier) (.StickY (Class|PlayerController|GetInputAnalogStickState (Variables|Default|GetRunningPC) "CAS_LeftStick"))))) false false)
  (Transformation|SetActorRotation _self_2 (Math|Rotator|MakeRotator (.roll _returnvalue) (Math|Float|Clamp(Float) (+ (.pitch _returnvalue) (* (* _sticky _gamepad_rotation_multiplier) -1.0)) -89.0 89.0) (+ (.yaw _returnvalue) (* _stickx _gamepad_rotation_multiplier))))
  (if (or (Game|Player|WasInputKeyJustPressed _runningpc_4 "Gamepad_LeftTriggerAxis") (Game|Player|WasInputKeyJustPressed _runningpc_4 _key_movedown))
    (bind _returnvalue_7 (Utilities|Time|SetTimerbyEvent (delegate Custom|Event%20FlyDown) 0.001 true)))
  (if (or (Class|PlayerController|WasInputKeyJustReleased _runningpc_6 "Gamepad_LeftTriggerAxis") (Class|PlayerController|WasInputKeyJustReleased _runningpc_6 _key_movedown))
    (Utilities|Time|ClearandInvalidateTimerbyHandle _returnvalue_7))
  (if (or (Game|Player|WasInputKeyJustPressed _runningpc_5 "Gamepad_RightTriggerAxis") (Game|Player|WasInputKeyJustPressed _runningpc_5 _key_moveup))
    (bind _returnvalue_8 (Utilities|Time|SetTimerbyEvent (delegate Custom|Event%20FlyUp) 0.001 true)))
  (if (or (Class|PlayerController|WasInputKeyJustReleased _runningpc_3 "Gamepad_RightTriggerAxis") (Class|PlayerController|WasInputKeyJustReleased _runningpc_3 _key_moveup))
    (Utilities|Time|ClearandInvalidateTimerbyHandle _returnvalue_8))
  (if (Game|Player|WasInputKeyJustPressed (Variables|Default|GetRunningPC) (Variables|Default|GetKey_ResetRoll))
    (Transformation|SetActorRotation _self_3 (Math|Rotator|MakeRotator 0.0 (.pitch _returnvalue_2) (.yaw _returnvalue_2)))))

(event Custom|Event%20KeyRight
  (bind _self self)
  (Transformation|SetActorLocation _self (+ (Transformation|GetActorLocation _self) (* (Math|Vector|GetRightVector (Transformation|GetActorRotation _self)) (Variables|Default|GetMovement%20Multiplier))) false false))

(event Custom|Event%20KeyLeft
  (bind _self self)
  (Transformation|SetActorLocation _self (+ (Transformation|GetActorLocation _self) (* (Math|Vector|GetRightVector (Transformation|GetActorRotation _self)) (* (Variables|Default|GetMovement%20Multiplier) -1.0))) false false))

(event Custom|Event%20ForceStop_KeyRight
  (bind _self self)
  (bind _self_2 self)
  (bind _self_3 self)
  (bind _self_4 self)
  (bind _self_5 self)
  (bind _key_moveleft (Variables|Default|GetKey_MoveLeft))
  (bind _runningpc (Variables|Default|GetRunningPC))
  (bind _key_moveup (Variables|Default|GetKey_MoveUp))
  (bind _key_movedown (Variables|Default|GetKey_MoveDown))
  (bind _runningpc_2 (Variables|Default|GetRunningPC))
  (bind _rotation_multiplier (Variables|Default|GetRotation%20Multiplier))
  (bind _runningpc_3 (Variables|Default|GetRunningPC))
  (bind _gamepad_rotation_multiplier (Variables|Default|GetGamepad%20Rotation%20Multiplier))
  (bind _runningpc_4 (Variables|Default|GetRunningPC))
  (bind _runningpc_5 (Variables|Default|GetRunningPC))
  (bind _runningpc_6 (Variables|Default|GetRunningPC))
  (bind _returnvalue (Transformation|GetActorRotation _self_2))
  (bind (_stickx _sticky) (Class|PlayerController|GetInputAnalogStickState _runningpc "CAS_RightStick"))
  (bind _returnvalue_2 (Transformation|GetActorRotation _self_3))
  (bind _returnvalue_3 (Transformation|GetActorRotation _self_4))
  (bind (_deltax _deltay) (Class|PlayerController|GetInputMouseDelta _runningpc_2))
  (Utilities|Time|ClearandInvalidateTimerbyHandle (stale Custom|Event%20ForceStop_KeyBack _returnvalue_4))
  (if (Game|Player|WasInputKeyJustPressed (Variables|Default|GetRunningPC) _key_moveleft)
    (bind _returnvalue_4 (Utilities|Time|SetTimerbyEvent (delegate Custom|Event%20KeyLeft) 0.001 true)))
  (if (Class|PlayerController|WasInputKeyJustReleased (Variables|Default|GetRunningPC) _key_moveleft)
    (Utilities|Time|ClearandInvalidateTimerbyHandle _returnvalue_4))
  (Transformation|SetActorRotation _self_4 (Math|Rotator|MakeRotator (.roll _returnvalue_3) (Math|Float|Clamp(Float) (+ (.pitch _returnvalue_3) (* _deltay _rotation_multiplier)) -89.0 89.0) (+ (.yaw _returnvalue_3) (* _deltax _rotation_multiplier))))
  (Transformation|SetActorLocation _self_5 (+ (Transformation|GetActorLocation _self_5) (* (Math|Vector|GetRightVector (Transformation|GetActorRotation _self_5)) (* (Variables|Default|GetGamepad%20Movement%20Multiplier) (.StickX (Class|PlayerController|GetInputAnalogStickState (Variables|Default|GetRunningPC) "CAS_LeftStick"))))) false false)
  (Transformation|SetActorLocation _self (+ (Transformation|GetActorLocation _self) (* (Math|Vector|GetForwardVector (Transformation|GetActorRotation _self)) (* (Variables|Default|GetGamepad%20Movement%20Multiplier) (.StickY (Class|PlayerController|GetInputAnalogStickState (Variables|Default|GetRunningPC) "CAS_LeftStick"))))) false false)
  (Transformation|SetActorRotation _self_2 (Math|Rotator|MakeRotator (.roll _returnvalue) (Math|Float|Clamp(Float) (+ (.pitch _returnvalue) (* (* _sticky _gamepad_rotation_multiplier) -1.0)) -89.0 89.0) (+ (.yaw _returnvalue) (* _stickx _gamepad_rotation_multiplier))))
  (if (or (Game|Player|WasInputKeyJustPressed _runningpc_4 "Gamepad_LeftTriggerAxis") (Game|Player|WasInputKeyJustPressed _runningpc_4 _key_movedown))
    (bind _returnvalue_5 (Utilities|Time|SetTimerbyEvent (delegate Custom|Event%20FlyDown) 0.001 true)))
  (if (or (Class|PlayerController|WasInputKeyJustReleased _runningpc_6 "Gamepad_LeftTriggerAxis") (Class|PlayerController|WasInputKeyJustReleased _runningpc_6 _key_movedown))
    (Utilities|Time|ClearandInvalidateTimerbyHandle _returnvalue_5))
  (if (or (Game|Player|WasInputKeyJustPressed _runningpc_5 "Gamepad_RightTriggerAxis") (Game|Player|WasInputKeyJustPressed _runningpc_5 _key_moveup))
    (bind _returnvalue_6 (Utilities|Time|SetTimerbyEvent (delegate Custom|Event%20FlyUp) 0.001 true)))
  (if (or (Class|PlayerController|WasInputKeyJustReleased _runningpc_3 "Gamepad_RightTriggerAxis") (Class|PlayerController|WasInputKeyJustReleased _runningpc_3 _key_moveup))
    (Utilities|Time|ClearandInvalidateTimerbyHandle _returnvalue_6))
  (if (Game|Player|WasInputKeyJustPressed (Variables|Default|GetRunningPC) (Variables|Default|GetKey_ResetRoll))
    (Transformation|SetActorRotation _self_3 (Math|Rotator|MakeRotator 0.0 (.pitch _returnvalue_2) (.yaw _returnvalue_2)))))

(event EventOnBecomeViewTarget
  (params (PC :type Player%20Controller%20Object%20Reference))
  (CallFunction|EventUpdateRunningPC)
  (Variables|Default|SetbCurrentlyControlled true)
  (Development|PrintString "FreeCamera Became ViewTarget" true true "(R=0.000000,G=0.660000,B=1.000000,A=1.000000)" 1e+03))

(event EventOnEndViewTarget
  (params (PC :type Player%20Controller%20Object%20Reference))
  (Variables|Default|SetbCurrentlyControlled false)
  (CallFunction|ForceStopAllMovement)
  (Development|PrintString "FreeCamera No Longer ViewTarget" true true "(R=0.000000,G=0.660000,B=1.000000,A=1.000000)" 1e+03))

(event EventTick
  (params (DeltaSeconds :type Float%20%28single-precision%29))
  (bind _self self)
  (bind _self_2 self)
  (bind _self_3 self)
  (bind _self_4 self)
  (bind _self_5 self)
  (bind _key_moveback (Variables|Default|GetKey_MoveBack))
  (bind _key_moveright (Variables|Default|GetKey_MoveRight))
  (bind _key_moveleft (Variables|Default|GetKey_MoveLeft))
  (bind _runningpc (Variables|Default|GetRunningPC))
  (bind _key_moveup (Variables|Default|GetKey_MoveUp))
  (bind _key_movedown (Variables|Default|GetKey_MoveDown))
  (bind _runningpc_2 (Variables|Default|GetRunningPC))
  (bind _rotation_multiplier (Variables|Default|GetRotation%20Multiplier))
  (bind _runningpc_3 (Variables|Default|GetRunningPC))
  (bind _gamepad_rotation_multiplier (Variables|Default|GetGamepad%20Rotation%20Multiplier))
  (bind _runningpc_4 (Variables|Default|GetRunningPC))
  (bind _runningpc_5 (Variables|Default|GetRunningPC))
  (bind _runningpc_6 (Variables|Default|GetRunningPC))
  (bind _key_moveforward (Variables|Default|GetKey_MoveForward))
  (bind _returnvalue (Transformation|GetActorRotation _self_2))
  (bind (_stickx _sticky) (Class|PlayerController|GetInputAnalogStickState _runningpc "CAS_RightStick"))
  (bind _returnvalue_2 (Transformation|GetActorRotation _self_3))
  (bind _returnvalue_3 (Transformation|GetActorRotation _self_4))
  (bind (_deltax _deltay) (Class|PlayerController|GetInputMouseDelta _runningpc_2))
  (if (Variables|Default|GetbCurrentlyControlled)
    (if (Game|Player|WasInputKeyJustPressed (Variables|Default|GetRunningPC) _key_moveforward)
      (bind _returnvalue_4 (Utilities|Time|SetTimerbyEvent (delegate Custom|Event%20KeyForward) 0.001 true)))
    (if (Class|PlayerController|WasInputKeyJustReleased (Variables|Default|GetRunningPC) _key_moveforward)
      (Utilities|Time|ClearandInvalidateTimerbyHandle _returnvalue_4))
    (if (Game|Player|WasInputKeyJustPressed (Variables|Default|GetRunningPC) _key_moveback)
      (bind _returnvalue_5 (Utilities|Time|SetTimerbyEvent (delegate Custom|Event%20KeyBack) 0.001 true)))
    (if (Class|PlayerController|WasInputKeyJustReleased (Variables|Default|GetRunningPC) _key_moveback)
      (Utilities|Time|ClearandInvalidateTimerbyHandle _returnvalue_5))
    (if (Game|Player|WasInputKeyJustPressed (Variables|Default|GetRunningPC) _key_moveright)
      (bind _returnvalue_6 (Utilities|Time|SetTimerbyEvent (delegate Custom|Event%20KeyRight) 0.001 true)))
    (if (Class|PlayerController|WasInputKeyJustReleased (Variables|Default|GetRunningPC) _key_moveright)
      (Utilities|Time|ClearandInvalidateTimerbyHandle _returnvalue_6))
    (if (Game|Player|WasInputKeyJustPressed (Variables|Default|GetRunningPC) _key_moveleft)
      (bind _returnvalue_7 (Utilities|Time|SetTimerbyEvent (delegate Custom|Event%20KeyLeft) 0.001 true)))
    (if (Class|PlayerController|WasInputKeyJustReleased (Variables|Default|GetRunningPC) _key_moveleft)
      (Utilities|Time|ClearandInvalidateTimerbyHandle _returnvalue_7))
    (Transformation|SetActorRotation _self_4 (Math|Rotator|MakeRotator (.roll _returnvalue_3) (Math|Float|Clamp(Float) (+ (.pitch _returnvalue_3) (* _deltay _rotation_multiplier)) -89.0 89.0) (+ (.yaw _returnvalue_3) (* _deltax _rotation_multiplier))))
    (Transformation|SetActorLocation _self_5 (+ (Transformation|GetActorLocation _self_5) (* (Math|Vector|GetRightVector (Transformation|GetActorRotation _self_5)) (* (Variables|Default|GetGamepad%20Movement%20Multiplier) (.StickX (Class|PlayerController|GetInputAnalogStickState (Variables|Default|GetRunningPC) "CAS_LeftStick"))))) false false)
    (Transformation|SetActorLocation _self (+ (Transformation|GetActorLocation _self) (* (Math|Vector|GetForwardVector (Transformation|GetActorRotation _self)) (* (Variables|Default|GetGamepad%20Movement%20Multiplier) (.StickY (Class|PlayerController|GetInputAnalogStickState (Variables|Default|GetRunningPC) "CAS_LeftStick"))))) false false)
    (Transformation|SetActorRotation _self_2 (Math|Rotator|MakeRotator (.roll _returnvalue) (Math|Float|Clamp(Float) (+ (.pitch _returnvalue) (* (* _sticky _gamepad_rotation_multiplier) -1.0)) -89.0 89.0) (+ (.yaw _returnvalue) (* _stickx _gamepad_rotation_multiplier))))
    (if (or (Game|Player|WasInputKeyJustPressed _runningpc_4 "Gamepad_LeftTriggerAxis") (Game|Player|WasInputKeyJustPressed _runningpc_4 _key_movedown))
      (bind _returnvalue_8 (Utilities|Time|SetTimerbyEvent (delegate Custom|Event%20FlyDown) 0.001 true)))
    (if (or (Class|PlayerController|WasInputKeyJustReleased _runningpc_6 "Gamepad_LeftTriggerAxis") (Class|PlayerController|WasInputKeyJustReleased _runningpc_6 _key_movedown))
      (Utilities|Time|ClearandInvalidateTimerbyHandle _returnvalue_8))
    (if (or (Game|Player|WasInputKeyJustPressed _runningpc_5 "Gamepad_RightTriggerAxis") (Game|Player|WasInputKeyJustPressed _runningpc_5 _key_moveup))
      (bind _returnvalue_9 (Utilities|Time|SetTimerbyEvent (delegate Custom|Event%20FlyUp) 0.001 true)))
    (if (or (Class|PlayerController|WasInputKeyJustReleased _runningpc_3 "Gamepad_RightTriggerAxis") (Class|PlayerController|WasInputKeyJustReleased _runningpc_3 _key_moveup))
      (Utilities|Time|ClearandInvalidateTimerbyHandle _returnvalue_9))
    (if (Game|Player|WasInputKeyJustPressed (Variables|Default|GetRunningPC) (Variables|Default|GetKey_ResetRoll))
      (Transformation|SetActorRotation _self_3 (Math|Rotator|MakeRotator 0.0 (.pitch _returnvalue_2) (.yaw _returnvalue_2))))))

(event EventBeginPlay
  (Utilities|Time|SetTimerbyEvent (delegate Custom|Event%20Update%20Running%20PC) 1.0 true))

(fn ConstructionScript)

(fn ForceStopAllMovement
  (CallFunction|EventForceStopKeyForward)
  (CallFunction|EventForceStopKeyBack)
  (CallFunction|EventForceStopKeyRight)
  (CallFunction|EventForceStopKeyLeft)
  (CallFunction|EventForceStopFlyDown)
  (CallFunction|EventForceStopFlyUp))