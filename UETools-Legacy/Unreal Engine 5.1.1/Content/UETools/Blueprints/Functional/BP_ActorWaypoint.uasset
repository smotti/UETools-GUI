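; BP_ActorWaypoint is a UETools waypoint actor that labels the actor it is attached to with a widget showing name and distance.
; On Init it caches its WBP_ActorWaypoint, passes in the UETools cheat manager reference and runs both updates.
; Looping timers then feed its location and the parent's name to the widget.
; An invalid parent triggers the widget's OnActorDestroyed and clears only the name timer.
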(event Custom|Event%20Update%20Distance
  (Default|UpdateDistance (Variables|Default|GetWBP%20Actor%20Waypoint) (Transformation|GetActorLocation self)))

(event Custom|Event%20Update%20Actor%20Info
  (bind _self self)
  (bind _returnvalue (Actor|GetAttachParentActor _self))
  (Utilities|IsValid _returnvalue
    (:Is%20Valid
      (Rendering|Components|TextRender|SetText (Variables|/Game/UETools/Widgets/Functional/WBP_ActorWaypoint.WBP_ActorWaypoint_C|GetTextBlock_ActorName (Variables|Default|GetWBP%20Actor%20Waypoint)) (Utilities|Text|ToText(String) (Utilities|String|ToString(Object) _returnvalue))))
    (:Is%20Not%20Valid
      (Default|OnActorDestroyed (Variables|Default|GetWBP%20Actor%20Waypoint))
      (Utilities|Time|ClearandInvalidateTimerbyHandle (stale Custom|Event%20Init _returnvalue)))))

(event Custom|Event%20Init
  (Utilities|FlowControl|Sequence
    (:then_0
      (bind _aswbp_actor_waypoint (Utilities|Casting|CastToWBP_ActorWaypoint (UserInterface|GetUserWidgetObject (Variables|Default|GetActorWaypointWidget))))
      (Variables|Default|SetWBP%20Actor%20Waypoint _aswbp_actor_waypoint))
    (:then_1
      (Default|UpdateCheatManagerRef (Variables|Default|GetWBP%20Actor%20Waypoint) (Variables|Default|GetUETools%20Cheat%20Manager%20Reference))
      (CallFunction|EventUpdateDistance)
      (CallFunction|EventUpdateActorInfo))
    (:then_2
      (Utilities|Time|SetTimerbyEvent (delegate Custom|Event%20Update%20Distance) (Variables|Default|GetUpdate%20Delay) true)
      (bind _returnvalue (Utilities|Time|SetTimerbyEvent (delegate Custom|Event%20Update%20Actor%20Info) (Variables|Default|GetUpdate%20Delay) true)))))

(fn ConstructionScript)