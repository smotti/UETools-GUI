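; BP_LevelStreamingManager is a manager actor that exposes level loading and streaming operations as callable events.
; Its events are thin wrappers around engine calls for streaming levels in and out, flushing streaming, opening a level by name and spawning level instances.
; Only the level instance event validates its input, skipping empty names.
; On BeginPlay it prints a long-lived debug message confirming its creation.
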(event EventBeginPlay
  (Development|PrintString "Level Streaming Manager Created" true true "(R=0.000000,G=0.660000,B=1.000000,A=1.000000)" 1e+06))

(event EventStreamLevelin
  (params (Level%20Name :type Name :default "None") (Make%20Visible%20After%20Load :type Boolean) (Should%20Block%20on%20Load :type Boolean))
  (Game|LoadStreamLevel(byName) Level%20Name Make%20Visible%20After%20Load Should%20Block%20on%20Load))

(event EventStreamLevelOut
  (params (Level%20Name :type Name :default "None") (Should%20Block%20on%20Unload :type Boolean))
  (Game|UnloadStreamLevel(byName) Level%20Name Should%20Block%20on%20Unload))

(event EventLoadLevelInstance
  (params (Level%20Name :type String) (Location :type Vector :default "0, 0, 0") (Rotation :type Rotator :default "0, 0, 0") (Optional%20Level%20Name%20Override :type String))
  (if (not (Utilities|Array|IsEmpty Level%20Name))
    (Class|LevelStreamingDynamic|LoadLevelInstance Level%20Name Location Rotation Optional%20Level%20Name%20Override)))

(event EventFlushLevelStreaming
  (Class|GameplayStatics|FlushLevelStreaming))

(event EventOpenLevel
  (params (Level%20Name :type Name :default "None") (Absolute :type Boolean) (Options :type String))
  (Game|OpenLevel(byName) Level%20Name Absolute Options))

(fn ConstructionScript)