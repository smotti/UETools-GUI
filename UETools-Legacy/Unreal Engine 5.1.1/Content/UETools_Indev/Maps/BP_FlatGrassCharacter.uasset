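; BP_FlatGrassCharacter is a simple player character, stored among the UETools_Indev maps, with movement, mouse look and a jump-like launch.
; Axis inputs move it along its forward and right vectors with forced input and feed mouse motion into controller yaw and pitch.
; The LaunchUp action calls LaunchCharacter along the actor's up vector, only while the movement mode is Walking or NavMesh Walking, so it cannot trigger mid-air.
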(event Input|ActionEvents|InputActionInputAction_LaunchUp
  (params (Key :type Key%20Structure :default "None"))
  (:Pressed
    (switch Utilities|FlowControl|Switch|SwitchonEMovementMode (Variables|/Script/Engine.CharacterMovementComponent|GetMovementMode (Variables|Character|GetCharacterMovement))
      (:MOVE_Walking
        _)
      (:MOVE_NavWalking
        _))
    (Character|LaunchCharacter (* (Transformation|GetActorUpVector) 650) false false)))

(event Input|AxisEvents|InputAxisInputAxis_ForwardVector
  (params (AxisValue :type Float%20%28single-precision%29))
  (Pawn|Input|AddMovementInput (Transformation|GetActorForwardVector) AxisValue true))

(event Input|AxisEvents|InputAxisInputAxis_RightVector
  (params (AxisValue :type Float%20%28single-precision%29))
  (Pawn|Input|AddMovementInput (Transformation|GetActorRightVector) AxisValue true))

(event Input|AxisEvents|InputAxisInputAxis_MouseHorizontal
  (params (AxisValue :type Float%20%28single-precision%29))
  (Pawn|Input|AddControllerYawInput AxisValue))

(event Input|AxisEvents|InputAxisInputAxis_MouseVertical
  (params (AxisValue :type Float%20%28single-precision%29))
  (Pawn|Input|AddControllerPitchInput AxisValue))

(fn ConstructionScript)